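; Player controller that turns Enhanced Input actions into movement, jumping and camera look for the player character.
; On BeginPlay it adds the IMC_Player mapping context.
; Move input follows the yaw of the BP_Player camera, ignoring pitch and roll, and requires a successful cast to BP_Player.
; Jump and look act directly on player character 0, with look feeding controller pitch and yaw.
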(event `self.ReceiveBeginPlay`
  ;[1 1 1] Mapping :3
  (`EnhancedInputSubsystemInterface.AddMappingContext` (subsystem `EnhancedInputLocalPlayerSubsystem`) "/Game/Input/IMC_Player.IMC_Player" 0 (struct)))

(event `EnhancedInput|/Game/Input/Action/IA_Move`
  (params (ActionValue :type "Vector2D Structure") (ElapsedSeconds :type "Float (double-precision)") (TriggeredSeconds :type "Float (double-precision)") (InputAction :type "InputAction Object Reference" :default "/Game/Input/Action/IA_Move.IA_Move"))
  (bind _returnvalue (`GameplayStatics.GetPlayerCharacter` 0))
  ;[1 1 1] MOOOOOVE :3
  (:`Triggered`
    (bind _asbp_player (cast `/Game/BP_Player` (`GameplayStatics.GetPlayerCharacter` 0)))
    (bind (_returnvalue_roll _returnvalue_pitch _returnvalue_yaw) (`KismetMathLibrary.BreakRotator` (`SceneComponent.K2_GetComponentRotation` (`/Game/BP_Player.Camera` _asbp_player))))
    (`Pawn.AddMovementInput` _returnvalue (`KismetMathLibrary.GetRightVector` (`KismetMathLibrary.MakeRotator` 0.0 0.0 _returnvalue_yaw)) ActionValue_Y false)
    (`Pawn.AddMovementInput` _returnvalue (`KismetMathLibrary.GetForwardVector` (`KismetMathLibrary.MakeRotator` 0.0 0.0 _returnvalue_yaw)) ActionValue_X false)))

(event `EnhancedInput|/Game/Input/Action/IA_Jump`
  (params (ActionValue :type Boolean) (ElapsedSeconds :type "Float (double-precision)") (TriggeredSeconds :type "Float (double-precision)") (InputAction :type "InputAction Object Reference" :default "/Game/Input/Action/IA_Jump.IA_Jump"))
  ;[1 1 1] Jump :3
  (:`Started`
    (`Character.Jump` (`GameplayStatics.GetPlayerCharacter` 0))))

(event `EnhancedInput|/Game/Input/Action/IA_Look`
  (params (ActionValue :type "Vector2D Structure") (ElapsedSeconds :type "Float (double-precision)") (TriggeredSeconds :type "Float (double-precision)") (InputAction :type "InputAction Object Reference" :default "/Game/Input/Action/IA_Look.IA_Look"))
  (bind _returnvalue (`GameplayStatics.GetPlayerCharacter` 0))
  ;[1 1 1] camera :3
  (:`Triggered`
    (bind _result (`/Engine/EditorBlueprintResources/StandardMacros.NegateFloat` ActionValue_Y)
      (:`  `
        (`Pawn.AddControllerPitchInput` _returnvalue _result)
        (`Pawn.AddControllerYawInput` _returnvalue ActionValue_X)))))

(fn `UserConstructionScript`)